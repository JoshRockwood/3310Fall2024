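; Pressure plate door that swings open while the player character or a static mesh object is on its trigger.
; DoorTrigger begin overlap plays the DoorRotation timeline, whose HingedDoor track sets the Door's relative yaw.
; End overlap reverses the timeline to close it.
; Overlaps are not counted, so any qualifying exit starts closing the door even if another occupant remains.
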(event `self.DoorTrigger.OnComponentBeginOverlap`
  (params (OverlappedComponent :type "PrimitiveComponent Object Reference") (OtherActor :type "Actor Object Reference") (OtherComp :type "PrimitiveComponent Object Reference") (OtherBodyIndex :type Integer) (bFromSweep :type Boolean) (SweepResult :type "HitResult Structure (by ref)"))
  (`|ExecutionSequence`
    (:`then_0`
      (cast `/Game/ThirdPerson/Blueprints/BP_ThirdPersonCharacter` OtherActor)
      (bind (_direction _hingeddoor) (`Timeline|DoorRotation` :!label _label)
        (:`Update`
          (`SceneComponent.K2_SetRelativeRotation` (`self.Door`) (`KismetMathLibrary.MakeRotator` 0.0 0.0 _hingeddoor) false false))))
    (:`then_1`
      (cast `StaticMeshComponent` OtherComp)
      (goto _label))))

(event `self.DoorTrigger.OnComponentEndOverlap`
  (params (OverlappedComponent :type "PrimitiveComponent Object Reference") (OtherActor :type "Actor Object Reference") (OtherComp :type "PrimitiveComponent Object Reference") (OtherBodyIndex :type Integer))
  (`|ExecutionSequence`
    (:`then_0`
      (cast `/Game/ThirdPerson/Blueprints/BP_ThirdPersonCharacter` OtherActor)
      (goto _label :!via `Reverse`))
    (:`then_1`
      (cast `StaticMeshComponent` OtherComp)
      (goto _label :!via `Reverse`))))

(fn `UserConstructionScript`)