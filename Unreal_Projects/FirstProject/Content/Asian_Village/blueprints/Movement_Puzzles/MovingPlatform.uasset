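; MovingPlatform is a platform actor for movement puzzles that travels along a path of three points.
; Its construction script builds the InterpToMovement component's control points from three location variables, all relative to the starting position.
; It also copies the Duration variable into that component, which handles the motion without any event graph logic in this file.
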(fn `UserConstructionScript`
  (bind _interptomovement (`self.InterpToMovement`))
  (set `InterpToMovementComponent.ControlPoints` (`|MakeArray` (make `InterpControlPoint` (`self.Location01`)) (make `InterpControlPoint` (`self.Location02`)) (make `InterpControlPoint` (`self.Location03`))) _interptomovement)
  (set `InterpToMovementComponent.Duration` (`self.Duration`) _interptomovement))