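; BP_Teleport_2 is a movement-puzzle teleporter that sends the player character or overlapping static mesh components to an exit point.
; Overlapping TeleportTrigger teleports BP_ThirdPersonCharacter to ExitTeleport's location after DelayTime, resetting its rotation to zero.
; A parallel sequence branch moves any overlapping StaticMeshComponent there immediately, without sweep.
; Each path plays a 2D teleporter sound once the move is made.
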(event `self.TeleportTrigger.OnComponentBeginOverlap`
  (params (OverlappedComponent :type "PrimitiveComponent Object Reference") (OtherActor :type "Actor Object Reference") (OtherComp :type "PrimitiveComponent Object Reference") (OtherBodyIndex :type Integer) (bFromSweep :type Boolean) (SweepResult :type "HitResult Structure (by ref)"))
  (bind _returnvalue (`SceneComponent.K2_GetComponentLocation` (`self.ExitTeleport`)))
  (`|ExecutionSequence`
    (:`then_0`
      (bind _asbp_third_person_character (cast `/Game/ThirdPerson/Blueprints/BP_ThirdPersonCharacter` OtherActor))
      (`KismetSystemLibrary.Delay` (`self.DelayTime`))
      (`self.K2_TeleportTo` :`self` _asbp_third_person_character :`DestLocation` _returnvalue)
      (`GameplayStatics.PlaySound2D` "/Game/Asian_Village/SoundFX/Valorant_Teleporter_Sound_Effect.Valorant_Teleporter_Sound_Effect" 1.0 1.0 0.0 null null))
    (:`then_1`
      (bind _asstatic_mesh_component (cast `StaticMeshComponent` OtherComp))
      (`SceneComponent.K2_SetWorldLocation` _asstatic_mesh_component _returnvalue false true)
      (`GameplayStatics.PlaySound2D` "/Game/Asian_Village/SoundFX/Valorant_Teleporter_Sound_Effect.Valorant_Teleporter_Sound_Effect" 1.0 1.0 0.0 null null))))

(fn `UserConstructionScript`)