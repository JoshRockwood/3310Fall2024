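; BP_TurretRandomProjectile is a turret that repeatedly spawns a randomly chosen projectile.
; BeginPlay starts an endless Delay loop that waits SpawnDuration, then spawns one of the first three AmmoTypes classes at ProjectileSpawnPoint's location and rotation.
; Each spawn is scaled by ProjectileScale and given ProjectileLifeSpan as its lifespan.
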(event `self.ReceiveBeginPlay`
  (bind (_returnvalue_location _returnvalue_rotation) (`KismetMathLibrary.BreakTransform` (`SceneComponent.K2_GetComponentToWorld` (`self.ProjectileSpawnPoint`))))
  (`KismetSystemLibrary.Delay` (`self.SpawnDuration`) :!label _label)
  (bind _returnvalue (`|SpawnActorFromClass` (`|GetArrayItem` (`self.AmmoTypes`) (`KismetMathLibrary.RandomIntegerInRange` 0 2)) (`KismetMathLibrary.MakeTransform` _returnvalue_location _returnvalue_rotation (`KismetMathLibrary.Conv_DoubleToVector` (`self.ProjectileScale`))) "Undefined" "MultiplyWithRoot" null null))
  (`self.SetLifeSpan` _returnvalue (`self.ProjectileLifeSpan`))
  (goto _label))

(fn `UserConstructionScript`)