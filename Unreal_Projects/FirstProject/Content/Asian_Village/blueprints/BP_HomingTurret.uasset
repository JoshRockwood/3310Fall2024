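; BP_HomingTurret is a turret actor that turns toward the player character and fires projectiles once it spots them.
; PawnSensing filters for BP_ThirdPersonCharacter, and each sighting snaps the actor's rotation to face that pawn.
; The sighting also enters a self-looping Delay that spawns BP_TurretProjectile at the Arrow's transform with a set lifespan.
; The loop has no exit, so firing continues after sight is lost.
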(event `self.PawnSensing.OnSeePawn`
  (params (Pawn :type "Pawn Object Reference"))
  (cast `/Game/ThirdPerson/Blueprints/BP_ThirdPersonCharacter` Pawn)
  (`self.K2_SetActorRotation` (`KismetMathLibrary.FindLookAtRotation` (`self.K2_GetActorLocation`) (`self.K2_GetActorLocation` Pawn)))
  (`KismetSystemLibrary.Delay` (`self.Delay`) :!label _label)
  (bind _returnvalue (`|SpawnActorFromClass` "/Game/Asian_Village/blueprints/BP_TurretProjectile.BP_TurretProjectile_C" (`SceneComponent.K2_GetComponentToWorld` (`self.Arrow`)) "Undefined" "MultiplyWithRoot" null null))
  (`self.SetLifeSpan` _returnvalue (`self.ProjectileLifeSpan`))
  (goto _label))

(fn `UserConstructionScript`)